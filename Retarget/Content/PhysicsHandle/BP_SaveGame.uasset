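; SaveGame object for the PhysicsHandle game that stores the player's stone count and world location.
; SaveData copies StoneCount from the pawn's BP_PH_PlayerState and records the pawn's actor location.
; LoadData passes the saved count to the player state's ReloadStone and moves the pawn to the saved location without sweeping.
; Both functions do nothing if the PlayerState cast fails, and neither performs slot read or write itself.
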(fn `LoadData`
  (params (Pawn :type "Pawn Object Reference"))
  (bind _asbp_ph_player_state (cast `/Game/PhysicsHandle/BP_PH_PlayerState` (`Pawn.PlayerState` Pawn)))
  (`/Game/PhysicsHandle/BP_PH_PlayerState.ReloadStone` _asbp_ph_player_state (`self.StoneCount`))
  (`Actor.K2_SetActorLocation` Pawn (`self.PlayerLoc`) false false))

(fn `SaveData`
  (params (Pawn :type "Pawn Object Reference"))
  (bind _asbp_ph_player_state (cast `/Game/PhysicsHandle/BP_PH_PlayerState` (`Pawn.PlayerState` Pawn)))
  (set `self.StoneCount` (`/Game/PhysicsHandle/BP_PH_PlayerState.StoneCount` _asbp_ph_player_state))
  (set `self.PlayerLoc` (`Actor.K2_GetActorLocation` Pawn)))